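; BP_ControlButton is a button that opens its referenced Gate while something overlaps its trigger volume and closes it when the volume empties.
; Begin and end overlap events keep a count of overlapping actors, so only the first arrival calls Open and only the last departure calls Close.
; Both calls are skipped when the Gate reference is not valid.
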(event OnComponentBeginOverlap(TriggerVolume)
  (params (OverlappedComponent :type Primitive%20Component%20Object%20Reference) (OtherActor :type Actor%20Object%20Reference) (OtherComp :type Primitive%20Component%20Object%20Reference) (OtherBodyIndex :type Integer) (bFromSweep :type Boolean) (SweepResult :type Hit%20Result%20Structure%20%28by%20ref%29))
  (if (and (== (Variables|Default|GetOverlappedActors) 0) (Utilities|IsValid (Variables|Default|GetGate)))
    (Default|Open (Variables|Default|GetGate)))
  (Math|Integer|IncrementInt (Variables|Default|GetOverlappedActors)))

(event OnComponentEndOverlap(TriggerVolume)
  (params (OverlappedComponent :type Primitive%20Component%20Object%20Reference) (OtherActor :type Actor%20Object%20Reference) (OtherComp :type Primitive%20Component%20Object%20Reference) (OtherBodyIndex :type Integer))
  (bind _result (Math|Integer|DecrementInt (Variables|Default|GetOverlappedActors))
    (:%20%20
      (if (and (== _result 0) (Utilities|IsValid (Variables|Default|GetGate)))
        (Default|Close (Variables|Default|GetGate))))))

(event EventBeginPlay)

(event Collision|EventActorBeginOverlap
  (params (OtherActor :type Actor%20Object%20Reference)))

(event EventTick
  (params (DeltaSeconds :type Float%20%28single-precision%29)))

(fn ConstructionScript)