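; Test actor for physical animation on a blob skeletal mesh driven by ABP_Big_CuBlob1.
; On BeginPlay it assigns the selected physics asset, applies world-space physical animation settings below a chosen body and simulates those bodies, leaving that body itself unsimulated.
; Each tick it sets the physical animation strength from RelaxRate and passes two animations and a blend alpha to the Anim Blueprint.
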(event EventTick
  (params (DeltaSeconds :type Float%20%28single-precision%29))
  (Class|PhysicalAnimationComponent|SetStrengthMultiplyer (Variables|Default|GetPhysicalAnimation) (Variables|Default|GetRelaxRate))
  (bind _asabp_big_cu_blob_1 (Utilities|Casting|CastToABP_Big_CuBlob1 (Components|SkeletalMesh|GetAnimInstance (Variables|SkeletalMeshActor|GetSkeletalMeshComponent))))
  (Variables|/Game/Blob/Blueprints/ABP_Big_CuBlob1.ABP_Big_CuBlob1_C|SetSequence _asabp_big_cu_blob_1 (Variables|Default|GetAnimation%201))
  (Variables|/Game/Blob/Blueprints/ABP_Big_CuBlob1.ABP_Big_CuBlob1_C|SetSequence_0 _asabp_big_cu_blob_1 (Variables|Default|GetAnimation%202))
  (Variables|/Game/Blob/Blueprints/ABP_Big_CuBlob1.ABP_Big_CuBlob1_C|Setanimation%20blend%20alpha _asabp_big_cu_blob_1 (Variables|Default|GetAnimation%20Blend%20Alpha)))

(event Collision|EventActorBeginOverlap
  (params (OtherActor :type Actor%20Object%20Reference)))

(event EventBeginPlay
  (bind _skeletalmeshcomponent (Variables|SkeletalMeshActor|GetSkeletalMeshComponent))
  (bind _physicalanimation (Variables|Default|GetPhysicalAnimation))
  (bind _body_name (Variables|Default|GetBody%20Name))
  (Components|SkinnedMesh|SetPhysicsAsset (Variables|SkeletalMeshActor|GetSkeletalMeshComponent) (Variables|Default|GetSelect%20physical%20asset) false)
  (Class|PhysicalAnimationComponent|SetSkeletalMeshComponent _physicalanimation _skeletalmeshcomponent)
  (Class|PhysicalAnimationComponent|ApplyPhysicalAnimationSettingsBelow _physicalanimation _body_name (Utilities|Struct|MakePhysicalAnimationData false 1e+03 15.0 1e+03 3e+01) false)
  (Class|SkeletalMeshComponent|SetAllBodiesBelowSimulatePhysics _skeletalmeshcomponent _body_name true false))

(fn ConstructionScript)