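; Tentacle actor that turns to face a BP_Blob while it is inside its trigger volume.
; Overlap begin stores the blob as Target and sets IsAttacking; overlap end clears both.
; While attacking, Tick snaps the actor's yaw toward the target with a look-at rotation, preserving pitch and roll.
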(event OnComponentBeginOverlap(TriggerVolume)
  (params (OverlappedComponent :type Primitive%20Component%20Object%20Reference) (OtherActor :type Actor%20Object%20Reference) (OtherComp :type Primitive%20Component%20Object%20Reference) (OtherBodyIndex :type Integer) (bFromSweep :type Boolean) (SweepResult :type Hit%20Result%20Structure%20%28by%20ref%29))
  (bind _asbp_blob (Utilities|Casting|CastToBP_Blob OtherActor))
  (Variables|Default|SetTarget _asbp_blob)
  (Variables|Default|SetIsAttacking%20 true))

(event OnComponentEndOverlap(TriggerVolume)
  (params (OverlappedComponent :type Primitive%20Component%20Object%20Reference) (OtherActor :type Actor%20Object%20Reference) (OtherComp :type Primitive%20Component%20Object%20Reference) (OtherBodyIndex :type Integer))
  (Utilities|Casting|CastToBP_Blob OtherActor)
  (Variables|Default|SetTarget 0)
  (Variables|Default|SetIsAttacking%20 false))

(event EventTick
  (params (DeltaSeconds :type Float%20%28single-precision%29))
  (bind _returnvalue (Transformation|GetActorRotation))
  (if (Variables|Default|GetIsAttacking%20)
    (Transformation|SetActorRotation (Math|Rotator|MakeRotator (.roll _returnvalue) (.pitch _returnvalue) (.yaw (Math|Rotator|FindLookatRotation (Transformation|GetActorLocation) (Transformation|GetActorLocation (Variables|Default|GetTarget))))))))

(fn ConstructionScript)