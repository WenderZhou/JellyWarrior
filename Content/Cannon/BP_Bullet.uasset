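; BP_Bullet is a cannon projectile that breaks Chaos destructibles where it lands.
; When its static mesh hits something, it spawns an FS_MasterField at the impact point, configures it as a short-lived radial field and triggers it.
; If ShouldPlaySound is set, it also spawns BP_Explosion at its own transform, then destroys itself.
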(event OnComponentHit(StaticMeshComponent)
  (params (HitComponent :type Primitive%20Component%20Object%20Reference) (OtherActor :type Actor%20Object%20Reference) (OtherComp :type Primitive%20Component%20Object%20Reference) (NormalImpulse :type Vector :default "0, 0, 0") (Hit :type Hit%20Result%20Structure%20%28by%20ref%29))
  (bind (_bblockinghit _binitialoverlap _time _distance _location _impactpoint _normal _impactnormal) (Collision|BreakHitResult Hit))
  (bind _returnvalue (Math|Conversions|ToTransform(Vector) _impactpoint))
  (bind _returnvalue_2 (Game|SpawnActorfromClass "/Engine/EditorResources/FieldNodes/FS_MasterField.FS_MasterField_C" (Math|Transform|MakeTransform (.location _returnvalue) (.rotation _returnvalue) "2.000000,2.000000,2.000000") "Undefined" "MultiplyWithRoot" 0 0))
  (Variables|Default|SetChaosImpactFieldRef _returnvalue_2)
  (Variables|/Engine/EditorResources/FieldNodes/FS_MasterField.FS_MasterField_C|SetActivationType (Variables|Default|GetChaosImpactFieldRef) "NewEnumerator4")
  (Variables|/Engine/EditorResources/FieldNodes/FS_MasterField.FS_MasterField_C|SetFieldLifespan (Variables|Default|GetChaosImpactFieldRef) 0.1)
  (Variables|/Engine/EditorResources/FieldNodes/FS_MasterField.FS_MasterField_C|SetRadial%20Magnitude (Variables|Default|GetChaosImpactFieldRef) 1.5e+02)
  (Default|CETrigger (Variables|Default|GetChaosImpactFieldRef))
  (if (Variables|Default|GetShouldPlaySound)
    (Game|SpawnActorfromClass "/Game/Cannon/BP_Explosion.BP_Explosion_C" (Transformation|GetActorTransform) "Undefined" "MultiplyWithRoot" 0 0))
  (Actor|DestroyActor))

(event EventBeginPlay)

(fn ConstructionScript)