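; BP_CheckPoint is a checkpoint actor that saves when triggered and can respawn the player as a BP_Blob.
; Overlapping its TriggerVolume calls Save on the other actor and, on success, plays a timeline that moves the flag.
; Recover destroys and respawns any valid linked Boat at that boat's SpawnTransform, then spawns a blob offset from the checkpoint and has player controller 0 possess it.
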(event OnComponentBeginOverlap(TriggerVolume)
  (params (OverlappedComponent :type Primitive%20Component%20Object%20Reference) (OtherActor :type Actor%20Object%20Reference) (OtherComp :type Primitive%20Component%20Object%20Reference) (OtherBodyIndex :type Integer) (bFromSweep :type Boolean) (SweepResult :type Hit%20Result%20Structure%20%28by%20ref%29))
  (bind _returnvalue (Class|CheckPoint|Save OtherActor))
  (if _returnvalue
    (bind _flaglocation (Timeline|Timeline Play)
      (:Update
        (Transformation|SetRelativeLocation (Variables|Default|GetFlag) _flaglocation false false)))))

(event EventBeginPlay)

(event Collision|EventActorBeginOverlap
  (params (OtherActor :type Actor%20Object%20Reference)))

(event EventTick
  (params (DeltaSeconds :type Float%20%28single-precision%29)))

(fn ConstructionScript)

(fn Recover
  (CallFunction|RocoverBoat)
  (bind _returnvalue (Game|SpawnActorfromClass "/Game/Blob/BP_Blob.BP_Blob_C" (Math|Transform|MakeTransform (+ (Transformation|GetActorLocation) "0.000000,-200.000000,400.000000") "0, 0, 0" "1.000000,1.000000,1.000000") "Undefined" "MultiplyWithRoot" 0 0))
  (Pawn|Possess (Game|GetPlayerController 0) _returnvalue))

(fn RocoverBoat
  (Utilities|IsValid (Variables|Default|GetBoat)
    (:Is%20Valid
      (Variables|Default|SetBoatSpawnTransform (Variables|/Game/Boat/BP_Boat.BP_Boat_C|GetSpawnTransform (Variables|Default|GetBoat)))
      (Actor|DestroyActor (Variables|Default|GetBoat))
      (bind _returnvalue (Game|SpawnActorfromClass "/Game/Boat/BP_Boat.BP_Boat_C" (Variables|Default|GetBoatSpawnTransform) "Undefined" "MultiplyWithRoot" 0 0))
      (Variables|Default|SetBoat _returnvalue))))