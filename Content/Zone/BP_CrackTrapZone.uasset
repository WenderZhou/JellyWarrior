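; Trap zone that fires a Chaos physics impact and topples a fake checkpoint when the blob enters it.
; When a BP_Blob capsule overlaps the box, it spawns a short-lived FS_MasterField at the zone's location and triggers it with a radial force.
; It also turns on physics simulation for the referenced FakeCheckPoint's flagpole and plays a crack sound, with no guard against retriggering.
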(event OnComponentBeginOverlap(Box)
  (params (OverlappedComponent :type Primitive%20Component%20Object%20Reference) (OtherActor :type Actor%20Object%20Reference) (OtherComp :type Primitive%20Component%20Object%20Reference) (OtherBodyIndex :type Integer) (bFromSweep :type Boolean) (SweepResult :type Hit%20Result%20Structure%20%28by%20ref%29))
  (Utilities|Casting|CastToCapsuleComponent OtherComp)
  (Utilities|Casting|CastToBP_Blob OtherActor)
  (bind _returnvalue (Game|SpawnActorfromClass "/Engine/EditorResources/FieldNodes/FS_MasterField.FS_MasterField_C" (Math|Transform|MakeTransform (Transformation|GetActorLocation) "0, 0, 0" "2.000000,2.000000,2.000000") "Undefined" "MultiplyWithRoot" 0 0))
  (bind _output_get (Variables|Default|SetChaosImpactFieldRef _returnvalue))
  (Variables|/Engine/EditorResources/FieldNodes/FS_MasterField.FS_MasterField_C|SetActivationType (Variables|Default|GetChaosImpactFieldRef) "NewEnumerator4")
  (Variables|/Engine/EditorResources/FieldNodes/FS_MasterField.FS_MasterField_C|SetFieldLifespan (Variables|Default|GetChaosImpactFieldRef) 0.1)
  (Variables|/Engine/EditorResources/FieldNodes/FS_MasterField.FS_MasterField_C|SetRadial%20Magnitude (Variables|Default|GetChaosImpactFieldRef) 1.5e+02)
  (Default|CETrigger (Variables|Default|GetChaosImpactFieldRef))
  (Physics|SetSimulatePhysics (Variables|/Game/CheckPoint/BP_FakeCheckPoint.BP_FakeCheckPoint_C|GetSM_Flagpole (Variables|Default|GetFakeCheckPoint)) true)
  (Audio|PlaySoundatLocation "/Game/Cannon/Crack.Crack" "0, 0, 0" "0, 0, 0" 1.0 1.0 0.1 0 0 0 0))

(event EventBeginPlay)

(event Collision|EventActorBeginOverlap
  (params (OtherActor :type Actor%20Object%20Reference)))

(event EventTick
  (params (DeltaSeconds :type Float%20%28single-precision%29)))

(fn ConstructionScript)