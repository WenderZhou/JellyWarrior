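; BP_StopPhysicsZone is a trigger volume that freezes drawbridges once they enter it.
; When its Box component begins overlapping a BP_DrawBridge or BP_DrawBridge1 actor, it waits one second.
; It then turns off physics simulation on that actor's Bridge1 and Bridge2 components, using a separate cast branch for each bridge class.
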(event OnComponentBeginOverlap(Box)
  (params (OverlappedComponent :type Primitive%20Component%20Object%20Reference) (OtherActor :type Actor%20Object%20Reference) (OtherComp :type Primitive%20Component%20Object%20Reference) (OtherBodyIndex :type Integer) (bFromSweep :type Boolean) (SweepResult :type Hit%20Result%20Structure%20%28by%20ref%29))
  (bind _asbp_draw_bridge (Utilities|Casting|CastToBP_DrawBridge OtherActor)
    (:then
      (Utilities|FlowControl|Delay 1.0)
      (Physics|SetSimulatePhysics (Variables|/Game/Building/BP_DrawBridge.BP_DrawBridge_C|GetBridge1 _asbp_draw_bridge) false)
      (Physics|SetSimulatePhysics (Variables|/Game/Building/BP_DrawBridge.BP_DrawBridge_C|GetBridge2 _asbp_draw_bridge) false))
    (:CastFailed
      (bind _asbp_draw_bridge_1 (Utilities|Casting|CastToBP_DrawBridge1 OtherActor))
      (Utilities|FlowControl|Delay 1.0)
      (Physics|SetSimulatePhysics (Variables|/Game/Building/BP_DrawBridge1.BP_DrawBridge1_C|GetBridge1 _asbp_draw_bridge_1) false)
      (Physics|SetSimulatePhysics (Variables|/Game/Building/BP_DrawBridge1.BP_DrawBridge1_C|GetBridge2 _asbp_draw_bridge_1) false))))

(event EventBeginPlay)

(event Collision|EventActorBeginOverlap
  (params (OtherActor :type Actor%20Object%20Reference)))

(event EventTick
  (params (DeltaSeconds :type Float%20%28single-precision%29)))

(fn ConstructionScript)