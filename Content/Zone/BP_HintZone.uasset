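; BP_HintZone is a trigger zone that shows a hint to the player's blob after it lingers inside.
; When the BP_Blob's capsule component enters the Box, a one-shot timer starts using the configurable Time.
; When the timer fires, it queues Message on that blob's prompt system via PromptEnqueue.
; Leaving the box clears the timer, so brief visits show no hint.
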(event OnComponentBeginOverlap(Box)
  (params (OverlappedComponent :type Primitive%20Component%20Object%20Reference) (OtherActor :type Actor%20Object%20Reference) (OtherComp :type Primitive%20Component%20Object%20Reference) (OtherBodyIndex :type Integer) (bFromSweep :type Boolean) (SweepResult :type Hit%20Result%20Structure%20%28by%20ref%29))
  (bind _asbp_blob (Utilities|Casting|CastToBP_Blob OtherActor))
  (Utilities|Casting|CastToCapsuleComponent OtherComp)
  (bind _returnvalue (Utilities|Time|SetTimerbyEvent (delegate Custom|HintPrompt) (Variables|Default|GetTime)))
  (Variables|Default|SetTimerHandle _returnvalue))

(event OnComponentEndOverlap(Box)
  (params (OverlappedComponent :type Primitive%20Component%20Object%20Reference) (OtherActor :type Actor%20Object%20Reference) (OtherComp :type Primitive%20Component%20Object%20Reference) (OtherBodyIndex :type Integer))
  (Utilities|Casting|CastToBP_Blob OtherActor)
  (Utilities|Casting|CastToCapsuleComponent OtherComp)
  (Utilities|Time|ClearandInvalidateTimerbyHandle (Variables|Default|GetTimerHandle)))

(event Custom|HintPrompt
  (Class|Jelly|PromptEnqueue (stale OnComponentBeginOverlap(Box) _asbp_blob) (Variables|Default|GetMessage)))

(event EventBeginPlay)

(event Collision|EventActorBeginOverlap
  (params (OtherActor :type Actor%20Object%20Reference)))

(event EventTick
  (params (DeltaSeconds :type Float%20%28single-precision%29)))

(fn ConstructionScript)