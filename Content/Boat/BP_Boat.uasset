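; BP_Boat is a player-steerable boat driven by physics.
; The MoveForward axis applies force along the actor's forward vector, and MoveRight applies yaw torque, both to the Boat component.
; Both use acceleration change, so handling is independent of mass.
; BeginPlay stores the spawn transform, which nothing in these graphs reads back.
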(event Custom|MoveRight
  (params (Value :type Float%20%28double-precision%29))
  (Class|PrimitiveComponent|AddTorqueinDegrees (Variables|Default|GetBoat) (* Value "0.000000,0.000000,20.000000") "None" true))

(event Custom|MoveForward
  (params (Value :type Float%20%28double-precision%29))
  (Physics|AddForce (Variables|Default|GetBoat) (* Value (Transformation|GetActorForwardVector) 5e+02) "None" true))

(event EventBeginPlay
  (Variables|Default|SetSpawnTransform (Transformation|GetActorTransform)))

(fn ConstructionScript)